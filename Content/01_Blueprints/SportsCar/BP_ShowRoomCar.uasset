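; BP_ShowRoomCar is a drivable car Blueprint that maps player input to its vehicle movement component.
; Forward input applies full throttle at zero or above and proportional brake below zero, while steering and handbrake inputs pass straight through.
; The construction script creates a dynamic material instance of the first mesh slot and stores it as the chassis material.
; A helper function re-enables the crash sound flag and prints a debug string.
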(event EventBeginPlay)

(event Collision|EventActorBeginOverlap
  (params (OtherActor :type Actor%20Object%20Reference)))

(event Input|ActionEvents|InputActionHandbrake
  (params (Key :type Key%20Structure))
  (bind _vehiclemovementcomponent (Variables|Default|GetVehicleMovementComponent))
  ;[1 1 1] Movement control
  (:Pressed
    (Class|ChaosVehicleMovementComponent|SetHandbrakeInput _vehiclemovementcomponent true))
  (:Released
    (Class|ChaosVehicleMovementComponent|SetHandbrakeInput _vehiclemovementcomponent false)))

(event Input|AxisEvents|InputAxisMoveRight
  (params (AxisValue :type Float%20%28single-precision%29))
  ;[1 1 1] Movement control
  (Class|ChaosVehicleMovementComponent|SetSteeringInput (Variables|Default|GetVehicleMovementComponent) AxisValue))

(event Input|AxisEvents|InputAxisMoveForward
  (params (AxisValue :type Float%20%28single-precision%29))
  (bind _vehiclemovementcomponent (Variables|Default|GetVehicleMovementComponent))
  (bind _vehiclemovementcomponent_2 (Variables|Default|GetVehicleMovementComponent))
  ;[1 1 1] Movement control
  (if (>= AxisValue 0.0)
    (Class|ChaosVehicleMovementComponent|SetThrottleInput _vehiclemovementcomponent 1.0)
    (Class|ChaosVehicleMovementComponent|SetBrakeInput _vehiclemovementcomponent 0.0)
    (Utilities|FlowControl|DoOnce false)
    (else
      (Class|ChaosVehicleMovementComponent|SetBrakeInput _vehiclemovementcomponent_2 (* AxisValue -1.0))
      (Class|ChaosVehicleMovementComponent|SetThrottleInput _vehiclemovementcomponent_2 0.0))))

(fn ConstructionScript
  (bind _returnvalue (Rendering|Material|CreateDynamicMaterialInstance (Variables|Character|GetMesh) 0 0 "None" :!class /Script/Engine.PrimitiveComponent))
  (Variables|Default|SetChassis%20Material _returnvalue))

(fn ResetCrashSound
  (Variables|Default|SetCanCrashSound true)
  (Development|PrintString "Helyololo"))